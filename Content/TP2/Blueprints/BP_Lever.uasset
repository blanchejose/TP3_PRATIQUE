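; BP_Lever is a one-use lever that opens its linked TargetDoor when interacted with.
; Overlapping Characters toggle PromptText, which stays hidden once the lever is used.
; Interact sets Used and, only if TargetDoor is valid, calls OpenDoor and plays the TL_Lever timeline to swing HandlePivot by interpolating its relative rotation.
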(event `/Game/TP2/Blueprints/BPI_Interactable.Interact`
  (params (InstigatorPawn :type "Pawn Object Reference"))
  (bind _targetdoor (`self.TargetDoor`))
  (if (not (`self.bUsed`))
    (set `self.bUsed` true)
    (`SceneComponent.SetVisibility` (`self.PromptText`) false false)
    (`/Engine/EditorBlueprintResources/StandardMacros.IsValid` _targetdoor
      (:`Is Valid`
        (`/Game/TP2/Blueprints/BP_Door.OpenDoor` _targetdoor)
        (bind (_direction _alpha) (`Timeline|TL_Lever`)
          (:`Update`
            (`SceneComponent.K2_SetRelativeRotation` (`self.HandlePivot`) (`KismetMathLibrary.RLerp` (struct :`Pitch` 40.0) (struct :`Pitch` -40.0) _alpha) false false)))))))

(event `self.ReceiveActorEndOverlap`
  (params (OtherActor :type "Actor Object Reference"))
  (cast `Character` OtherActor)
  (`SceneComponent.SetVisibility` (`self.PromptText`) false false))

(event `self.ReceiveActorBeginOverlap`
  (params (OtherActor :type "Actor Object Reference"))
  (cast `Character` OtherActor)
  (if (not (`self.bUsed`))
    (`SceneComponent.SetVisibility` (`self.PromptText`) true false)))

(fn `UserConstructionScript`)