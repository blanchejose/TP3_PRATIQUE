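; Game mode for a collection level that ends once a player gathers the required coins and chests.
; On PostLogin it binds CheckVictory to the PS_Collector collectibles-changed event; meeting both thresholds prints a completion message and pauses the game.
; A separate EndGame function, not called by CheckVictory, shows WBP_EndScreen with the result, switches to UI-only input and pauses, guarded to run once.
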(event `self.K2_PostLogin`
  (params (NewPlayer :type "PlayerController Object Reference"))
  (bind _asps_collector (cast `/Game/TP2/Blueprints/PS_Collector` (`Controller.PlayerState` NewPlayer)))
  (add `/Game/TP2/Blueprints/PS_Collector.OnCollectiblesChanged` _asps_collector (delegate `CheckVictory`)))

(event `CheckVictory`
  (params (Coins :type Integer) (Chests :type Integer))
  (if (and (not (`self.bLevelComplete`)) (>= Coins (`self.RequiredCoins`)) (>= Chests (`self.RequiredChests`)))
    (set `self.bLevelComplete` true)
    (`KismetSystemLibrary.PrintString` "Niveau terminé!..." true true (struct :`G` 0.66 :`B` 1.0 :`A` 1.0) 15.0)
    (`GameplayStatics.SetGamePaused` true)))

(fn `EndGame`
  (params (bVictory :type Boolean))
  (bind _returnvalue (`GameplayStatics.GetPlayerController` 0))
  (if (not (`self.bGameEnded`))
    (set `self.bGameEnded` true)
    (bind _returnvalue_2 (`|CreateWidget` "/Game/TP3/UI/WBP_EndScreen.WBP_EndScreen_C" _returnvalue))
    (`/Game/TP3/UI/WBP_EndScreen.Setup` _returnvalue_2 bVictory)
    (`UserWidget.AddToViewport` _returnvalue_2 0)
    (set `PlayerController.bShowMouseCursor` true _returnvalue)
    (`WidgetBlueprintLibrary.SetInputMode_UIOnlyEx` _returnvalue _returnvalue_2)
    (`GameplayStatics.SetGamePaused` true)))

(fn `UserConstructionScript`)