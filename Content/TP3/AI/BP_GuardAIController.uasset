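; BP_GuardAIController is the AI controller for guard enemies, running the BT_Guard behavior tree when it possesses a pawn.
; Perception updates for the player character write the blackboard that drives the tree.
; A successful sense sets TargetActor and clears LastKnownLocation, while losing the player stores the stimulus location as LastKnownLocation and clears TargetActor.
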(event `self.AIPerception.OnTargetPerceptionUpdated`
  (params (Actor :type "Actor Object Reference") (Stimulus :type "AIStimulus Structure"))
  (bind (_age _expirationage _strength _stimuluslocation _receiverlocation _tag _bsuccessfullysensed) (break `AIStimulus` Stimulus))
  (bind _returnvalue (`AIBlueprintHelperLibrary.GetBlackboard` self))
  (if (== Actor (`GameplayStatics.GetPlayerCharacter` 0))
    (if _bsuccessfullysensed
      (`BlackboardComponent.SetValueAsObject` _returnvalue "TargetActor" Actor)
      (`BlackboardComponent.ClearValue` _returnvalue "LastKnownLocation")
      (else
        (`BlackboardComponent.SetValueAsVector` _returnvalue "LastKnownLocation" _stimuluslocation)
        (`BlackboardComponent.ClearValue` _returnvalue "TargetActor")))))

(event `self.ReceivePossess`
  (params (PossessedPawn :type "Pawn Object Reference"))
  (`self.RunBehaviorTree` "/Game/TP3/AI/BT_Guard.BT_Guard"))

(fn `UserConstructionScript`)